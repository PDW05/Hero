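; Player character Blueprint for the Chibi hero, with forward movement, yaw turning and attacks on A, S and D.
; Each key plays the same right-arm attack montage and spawns its own projectile class ahead of the character; D spawns two plus an explosion.
; Tick holds a weapon-socket trace for slash damage, but its branch ignores the montage check and is constant true, so that false-side logic never runs.
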(event EventTick
  (params (DeltaSeconds :type Float%20%28single-precision%29))
  (bind _weaponmesh (Variables|Default|GetWeaponMesh))
  ;[1 1 1] 근접 공격중인지 판별
  (Class|AnimInstance|MontageIsActive (Components|SkeletalMesh|GetAnimInstance (Variables|Character|GetMesh)) "/Game/ChibiHeroFemalePack/Animation/RightArmAttack_Anim_Montage.RightArmAttack_Anim_Montage")
  (if (not true)
    (Development|SetHiddeninGame (Variables|Default|GetBladeEffect) true false)
    ;[1 1 1] 트레이싱과 데미지처리
    (bind (_outhit _returnvalue) (Collision|LineTraceByChannel (Transformation|GetSocketLocation _weaponmesh "StartSocket") (Transformation|GetSocketLocation _weaponmesh "EndSocket") "TraceTypeQuery3" false 0 "None"))
    (if _returnvalue
      (Game|Damage|ApplyDamage (.HitActor (Collision|BreakHitResult _outhit)) (Variables|Default|GetSlashDamage) 0 0))))

(event Input|AxisEvents|InputAxisMoveForward
  (params (AxisValue :type Float%20%28single-precision%29))
  ;[1 1 1] 캐릭터 이동, 회전
  (Pawn|Input|AddMovementInput (Math|Vector|GetForwardVector (Class|KismetMathLibrary|MakeRot 0.0 (.Yaw (Class|KismetMathLibrary|BreakRot (Transformation|GetActorRotation))) 0.0)) AxisValue false))

(event Input|AxisEvents|InputAxisMoveRight
  (params (AxisValue :type Float%20%28single-precision%29))
  ;[1 1 1] 캐릭터 이동, 회전
  (Pawn|Input|AddControllerYawInput (* AxisValue 1.0)))

(event Input|KeyboardEvents|A
  (bind _returnvalue (Pawn|GetControlRotation :!class /Script/Engine.Pawn))
  ;[1 1 1] 원거리 공격
  (:Pressed
    (Game|SpawnActorfromClass "/Game/Bluprint/Projectile.Projectile_C" (Math|Transform|MakeTransform (+ (Transformation|GetActorLocation) (* (Math|Vector|GetForwardVector _returnvalue) 5e+01)) _returnvalue) (Variables|Default|Getspawn) 0 0)
    (Animation|Montage|MontagePlay (Components|SkeletalMesh|GetAnimInstance (Variables|Character|GetMesh)) "/Game/ChibiHeroFemalePack/Animation/RightArmAttack_Anim_Montage.RightArmAttack_Anim_Montage" 1.0)))

(event Input|KeyboardEvents|S
  (bind _returnvalue (Pawn|GetControlRotation :!class /Script/Engine.Pawn))
  ;[1 1 1] 근거리
  (:Pressed
    (Animation|Montage|MontagePlay (Components|SkeletalMesh|GetAnimInstance (Variables|Character|GetMesh)) "/Game/ChibiHeroFemalePack/Animation/RightArmAttack_Anim_Montage.RightArmAttack_Anim_Montage" 1.0)
    (Game|SpawnActorfromClass "/Game/Bluprint/Projectile_2.Projectile_2_C" (Math|Transform|MakeTransform (+ (* (Math|Vector|GetForwardVector _returnvalue) 5e+01) (Transformation|GetActorLocation)) _returnvalue) false 0 0)))

(event Input|KeyboardEvents|D
  ;[1 1 1] 근접 공격 애니메이션 재생
  (:Pressed
    (Animation|Montage|MontagePlay (Components|SkeletalMesh|GetAnimInstance (Variables|Character|GetMesh)) "/Game/ChibiHeroFemalePack/Animation/RightArmAttack_Anim_Montage.RightArmAttack_Anim_Montage" 1.0)))

(event Input|KeyboardEvents|D
  (bind _returnvalue (Transformation|GetActorLocation))
  (bind _returnvalue_2 (Pawn|GetControlRotation :!class /Script/Engine.Pawn))
  (bind _spawn (Variables|Default|Getspawn))
  (bind _returnvalue_3 (Math|Vector|GetForwardVector _returnvalue_2))
  (bind _returnvalue_4 (* _returnvalue_3 3e+02))
  (bind _returnvalue_5 (+ _returnvalue _returnvalue_4))
  (:Pressed
    (Utilities|FlowControl|Sequence
      (:then_0
        (Game|SpawnActorfromClass "/Game/Bluprint/Projctile_3.Projctile_3_C" (Math|Transform|MakeTransform _returnvalue_5 _returnvalue_2) _spawn 0 0)
        (Effects|SpawnEmitteratLocation "/Game/MyParticleSystem/P_Explosion.P_Explosion" _returnvalue_5 _returnvalue_2)
        (Animation|Montage|MontagePlay (Components|SkeletalMesh|GetAnimInstance (Variables|Character|GetMesh)) "/Game/ChibiHeroFemalePack/Animation/RightArmAttack_Anim_Montage.RightArmAttack_Anim_Montage" 1.0))
      (:then_1
        (Game|SpawnActorfromClass "/Game/Bluprint/Projctile_3.Projctile_3_C" (Math|Transform|MakeTransform (+ (* _returnvalue_3 2.9e+02) _returnvalue) _returnvalue_2) _spawn 0 0)))))

(fn ConstructionScript)